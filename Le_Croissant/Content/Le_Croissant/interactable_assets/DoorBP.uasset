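; Interactable door that the third-person character opens and closes with E once all collectables are gathered.
; A box trigger enables input while the character overlaps it and disables it on exit.
; On press, it checks CollectablesLeft on the game mode: at zero, a FlipFlop plays or reverses a timeline that swings the door's yaw, showing a success widget the first time.
; Otherwise it shows a fail widget.
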(event OnComponentBeginOverlap(Box)
  (params (OverlappedComponent :type Primitive%20Component%20Object%20Reference) (OtherActor :type Actor%20Object%20Reference) (OtherComp :type Primitive%20Component%20Object%20Reference) (OtherBodyIndex :type Integer) (bFromSweep :type Boolean) (SweepResult :type Hit%20Result%20Structure%20%28by%20ref%29))
  (Utilities|Casting|CastToBP_ThirdPersonCharacter OtherActor)
  (Input|EnableInput (Game|GetPlayerController 0)))

(event OnComponentEndOverlap(Box)
  (params (OverlappedComponent :type Primitive%20Component%20Object%20Reference) (OtherActor :type Actor%20Object%20Reference) (OtherComp :type Primitive%20Component%20Object%20Reference) (OtherBodyIndex :type Integer))
  (Utilities|Casting|CastToBP_ThirdPersonCharacter OtherActor)
  (Input|DisableInput (Game|GetPlayerController 0)))

(event Input|KeyboardEvents|E
  (params (Key :type Key%20Structure :default "None"))
  (:Pressed
    (bind _asbp_third_person_game_mode (Utilities|Casting|CastToBP_ThirdPersonGameMode (Game|GetGameMode)))
    (if (== (Variables|/Game/ThirdPerson/Blueprints/BP_ThirdPersonGameMode.BP_ThirdPersonGameMode_C|GetCollectablesLeft _asbp_third_person_game_mode) 0)
      (Utilities|FlowControl|FlipFlop
        (:A
          (if (Variables|Default|GetfirstTime)
            (bind _returnvalue (UserInterface|CreateWidget "/Game/Le_Croissant/interactable_assets/SuccessWidget.SuccessWidget_C"))
            (UserInterface|Viewport|AddtoViewport _returnvalue 0)
            (Variables|Default|SetfirstTime false)
            (bind _rotation (Timeline|open%20door Play)
              (:Update
                (Transformation|SetRelativeRotation (Variables|Default|GetDoor) (Math|Rotator|MakeRotator 0.0 0.0 (Math|Float|Lerp 0.0 115.0 _rotation)) false false)))
            (else
              (Timeline|open%20door Play))))
        (:B
          (Timeline|open%20door Reverse)))
      (else
        (bind _returnvalue_2 (UserInterface|CreateWidget "/Game/Le_Croissant/interactable_assets/FailWidget.FailWidget_C"))
        (UserInterface|Viewport|AddtoViewport _returnvalue_2 0)))))

(fn ConstructionScript)